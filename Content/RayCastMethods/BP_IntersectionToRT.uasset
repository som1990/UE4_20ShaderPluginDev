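; Actor that turns per-frame trace results into a mask texture and feeds it to a compute-shader height map simulation.
; Each Tick runs GenerateTrace and GenerateRTFromTrace, then passes the texture, delta time and trace U/V arrays to TargetCSTestSim.ComputeHeightMap.
; It also shows the generated texture on MeshComp through a dynamic material instance created in the construction script.
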(event EventBeginPlay)

(event Collision|EventActorBeginOverlap
  (params (OtherActor :type Actor%20Object%20Reference)))

(event EventTick
  (params (DeltaSeconds :type Float%20%28single-precision%29))
  (bind _mydynamicmaterial (Variables|Default|GetMyDynamicMaterial))
  ;[0.503 0.5281 1] Trace  and Mask Generation
  (bind (_u_outs _v_outs) (Class|IntersectiontoRT|GenerateTrace))
  (bind _generatedtexture (Class|IntersectiontoRT|GenerateRTfromTrace))
  (bind _output_get (Variables|Default|SetGeneratedTexture _generatedtexture))
  (Utilities|FlowControl|Sequence
    (:then_0
      ;[1 0.2977 0.5418] Send to Compute Shader Class Blueprint
      (Default|ComputeHeightMap (Variables|Default|GetTargetCSTestSim) _output_get DeltaSeconds _u_outs _v_outs))
    (:then_1
      ;[0.09861 1 0.154] Visualizing Texture
      (Rendering|Material|SetTextureParameterValue _mydynamicmaterial "DynamicTexture" _generatedtexture)
      (Rendering|Material|SetMaterial (Variables|Default|GetMeshComp) 0 _mydynamicmaterial))))

(fn ConstructionScript
  (bind _returnvalue (Rendering|Material|CreateDynamicMaterialInstance "/Game/RayCastMethods/MyDefaultMat.MyDefaultMat" "MyDynamicMat" :!class /Script/Engine.KismetMaterialLibrary))
  (Variables|Default|SetMyDynamicMaterial _returnvalue))