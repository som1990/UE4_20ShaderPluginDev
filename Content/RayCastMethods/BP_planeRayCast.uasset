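; Plane actor that scans object intersections every tick with TexSize line traces, apparently spaced along X and spanning its bounds in Y.
; Each ray is multi-traced forward and backward to catch entry and exit hits, which GenerateU normalizes against the Y extent.
; Hits are paired in opposite order into U0/U1 values, each pair overwriting that ray's Positions entry.
; Traces and forward hits are debug-displayed; nothing here consumes Positions beyond disabled debug printing.
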(event EventBeginPlay
  (bind _boxextent (Collision|GetActorBounds false))
  (bind (_x _y) (Math|Vector|BreakVector _boxextent))
  (Utilities|Array|Resize (Variables|Default|GetPositions) (Variables|Default|GettexSize))
  (Utilities|Array|Resize (Variables|Default|GetrayHitUVArray) (Variables|Default|GettexSize))
  (Variables|Default|SetySize _y)
  (Variables|Default|SetxSize _x))

(event Collision|EventActorBeginOverlap
  (params (OtherActor :type Actor%20Object%20Reference)))

(event EventTick
  (params (DeltaSeconds :type Float%20%28single-precision%29))
  (for _index (range 0 (- (Variables|Default|GettexSize) 1))
    (Variables|Default|Seti _index)
    (Utilities|FlowControl|Sequence
      (:then_0
        ;[1 1 1] Calculating Start/End Positions
        (Variables|Default|SetstartPos (.Start%20Point (Utilities|GenerateRayPositions (Variables|Default|Geti))))
        (Variables|Default|SetEndPos (.End%20Point (Utilities|GenerateRayPositions (Variables|Default|Geti)))))
      (:then_1
        (Utilities|Array|Clear (.U0 (Utilities|Struct|BreakRayHitUV (Utilities|Array|Get(acopy) (Variables|Default|GetrayHitUVArray) (Variables|Default|Geti)))))
        (bind (_outhits _returnvalue) (Class|KismetSystemLibrary|LineTraceMultiforObjects (Variables|Default|GetstartPos) (Variables|Default|GetEndPos) (Variables|Default|GetobjectType) true 0 "ForOneFrame" true "(R=1.000000,G=0.000000,B=0.000000,A=1.000000)" "(R=0.000000,G=1.000000,B=0.000000,A=1.000000)" 3.0))
        (bind _output_get (Variables|Default|SetbRay0Hit _returnvalue))
        (Variables|Default|Setu0Length (Utilities|Array|Length _outhits))
        (if _output_get
          (bind _array_element (Utilities|Array|ForEachLoopwithBreak _outhits)
            (:LoopBody
              (bind _out_u (CallFunction|GenerateU (.Location (Collision|BreakHitResult _array_element)) (Variables|Default|GetstartPos)))
              (Utilities|Array|SetArrayElem (.U0 (Utilities|Struct|BreakRayHitUV (Utilities|Array|Get(acopy) (Variables|Default|GetrayHitUVArray) (Variables|Default|Geti)))) 0 _out_u true)
              (Development|PrintString (Utilities|String|Append (Utilities|String|ToString(Float) (/ (.Distance (Collision|BreakHitResult _array_element)) (* (Variables|Default|GetySize) 2.0))) ",  " (Utilities|String|ToString(Float) _out_u)))))))
      (:then_2
        (Utilities|Array|Clear (.U1 (Utilities|Struct|BreakRayHitUV (Utilities|Array|Get(acopy) (Variables|Default|GetrayHitUVArray) (Variables|Default|Geti)))))
        (bind (_outhits_2 _returnvalue_2) (Class|KismetSystemLibrary|LineTraceMultiforObjects (Variables|Default|GetEndPos) (Variables|Default|GetstartPos) (Variables|Default|GetobjectType) true 0 "ForOneFrame" true "(R=1.000000,G=0.000000,B=0.000000,A=1.000000)" "(R=0.000000,G=1.000000,B=0.000000,A=1.000000)" 3.0))
        (bind _output_get_2 (Variables|Default|SetbRay1Hit _returnvalue_2))
        (Variables|Default|Setu1Length (Utilities|Array|Length _outhits_2))
        (if _output_get_2
          (bind (_array_element_2 _array_index) (Utilities|Array|ForEachLoopwithBreak _outhits_2)
            (:LoopBody
              (bind _out_u_2 (CallFunction|GenerateU (Variables|Default|GetEndPos) (.Location (Collision|BreakHitResult _array_element_2))))
              (Utilities|Array|SetArrayElem (.U1 (Utilities|Struct|BreakRayHitUV (Utilities|Array|Get(acopy) (Variables|Default|GetrayHitUVArray) (Variables|Default|Geti)))) _array_index (- 1.0 _out_u_2) true)))))
      (:then_3
        (if (> (Math|Integer|Max(Integer) (Variables|Default|Getu0Length) (Variables|Default|Getu1Length)) 0)
          (for _index_2 (range 0 (- (Math|Integer|Max(Integer) (Variables|Default|Getu0Length) (Variables|Default|Getu1Length)) 1))
            (Variables|Default|Setj _index_2)
            (Utilities|FlowControl|Sequence
              (:then_0
                (if (>= (- (- (Variables|Default|Getu1Length) 1) (Variables|Default|Getj)) 0)
                  (Variables|Default|SetfinalU1 (Utilities|Array|Get(acopy) (.U1 (Utilities|Struct|BreakRayHitUV (Utilities|Array|Get(acopy) (Variables|Default|GetrayHitUVArray) (Variables|Default|Geti)))) (- (- (Variables|Default|Getu1Length) 1) (Variables|Default|Getj))))
                  (else
                    (Variables|Default|SetfinalU1 1.0))))
              (:then_1
                (if (< (Variables|Default|Getj) (Variables|Default|Getu0Length))
                  (Variables|Default|SetfinalU0 (Utilities|Array|Get(acopy) (.U0 (Utilities|Struct|BreakRayHitUV (Utilities|Array|Get(acopy) (Variables|Default|GetrayHitUVArray) (Variables|Default|Geti)))) (Variables|Default|Getj)))
                  (else
                    (Variables|Default|SetfinalU0 0.0))))
              (:then_2
                (Utilities|Array|SetArrayElem (Variables|Default|GetPositions) (Variables|Default|Geti) (Math|Vector2D|MakeVector2D (Variables|Default|GetfinalU0) (Variables|Default|GetfinalU1))))))))
      (:then_4))))

(fn ConstructionScript)

(fn GenerateU
  (params (RayEnd :type Vector%20%28by%20ref%29) (RayStart :type Vector%20%28by%20ref%29))
  (bind _returnvalue (- RayEnd RayStart))
  (bind _ysize (Variables|Default|GetySize))
  (bind _y (Math|Vector|BreakVector _returnvalue))
  (bind _returnvalue_2 (* _ysize 2.0))
  (bind _returnvalue_3 (/ _y _returnvalue_2))
  (if (> _y 0.0)
    (if (<= _returnvalue_3 1.0)
      (return _returnvalue_3))))