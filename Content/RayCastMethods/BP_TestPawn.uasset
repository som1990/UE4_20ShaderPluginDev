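; BP_TestPawn is a test pawn that moves on input and measures its horizontal movement each frame.
; MoveForward and MoveRight axes feed movement input along the actor's forward and right vectors.
; Tick stores the XY distance from the previous frame's location in Mag, seeded at BeginPlay; nothing in this graph reads Mag.
; The distance is per frame and is not divided by delta time.
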(event EventBeginPlay
  (bind _returnvalue (Transformation|GetActorLocation))
  (bind _output_get (Variables|Default|SetPrevLoc (Math|Vector2D|MakeVector2D (.x _returnvalue) (.y _returnvalue))))
  (Variables|Default|SetcurLoc _output_get))

(event Collision|EventActorBeginOverlap
  (params (OtherActor :type Actor%20Object%20Reference)))

(event EventTick
  (params (DeltaSeconds :type Float%20%28single-precision%29))
  (bind _returnvalue (Transformation|GetActorLocation))
  (bind _output_get (Variables|Default|SetcurLoc (Math|Vector2D|MakeVector2D (.x _returnvalue) (.y _returnvalue))))
  (Variables|Default|Setmag (Math|Vector2D|Vector2DLength (- _output_get (Variables|Default|GetPrevLoc))))
  (Variables|Default|SetPrevLoc _output_get))

(event Input|AxisEvents|InputAxisMoveForward
  (params (AxisValue :type Float%20%28single-precision%29))
  (Pawn|Input|AddMovementInput (Transformation|GetActorForwardVector) AxisValue false))

(event Input|AxisEvents|InputAxisMoveRight
  (params (AxisValue :type Float%20%28single-precision%29))
  (Pawn|Input|AddMovementInput (Transformation|GetActorRightVector) AxisValue false))

(fn ConstructionScript)