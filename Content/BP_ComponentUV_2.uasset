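; BP_ComponentUV_2 is a movable pawn that feeds the UV coordinate of the point beneath it into a plane's material.
; Each tick it line-traces downward with complex collision and debug drawing, and checks whether it hit PlaneActor.
; On a hit, it calls CreateDynamicMaterialInstance on the hit component and writes the FindCollisionUV result to the "UV" vector parameter.
; MoveForward and MoveRight axes drive movement input; possession and UV print nodes are disconnected.
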(event EventBeginPlay)

(event EventTick
  (params (DeltaSeconds :type Float%20%28single-precision%29))
  (bind _returnvalue (Transformation|GetActorLocation))
  (bind _output_get (Variables|Default|SetRayDirection "0,0.000000,-1.000000"))
  (bind (_outhit _returnvalue_2) (Collision|LineTraceByChannel _returnvalue (+ (* _output_get (Variables|Default|GetTraceDistance)) _returnvalue) "TraceTypeQuery1" true 0 "ForDuration"))
  (if _returnvalue_2
    (if (== (.HitActor (Collision|BreakHitResult _outhit)) (Variables|Default|GetPlaneActor))
      (bind _returnvalue_3 (Rendering|Material|CreateDynamicMaterialInstance (.HitComponent (Collision|BreakHitResult _outhit)) 0 (Rendering|Material|GetMaterial (.HitComponent (Collision|BreakHitResult _outhit)) 0) "None" :!class /Script/Engine.PrimitiveComponent))
      (Rendering|Material|SetVectorParameterValue _returnvalue_3 "UV" (Utilities|Struct|MakeLinearColor (.X (Math|Vector2D|BreakVector2D (.UV (Class|GameplayStatics|FindCollisionUV _outhit)))) (.Y (Math|Vector2D|BreakVector2D (.UV (Class|GameplayStatics|FindCollisionUV _outhit)))) 0.0 1.0) :!class /Script/Engine.MaterialInstanceDynamic))))

(event Input|AxisEvents|InputAxisMoveRight
  (params (AxisValue :type Float%20%28single-precision%29))
  (Pawn|Input|AddMovementInput (Transformation|GetActorRightVector) AxisValue false))

(event Input|AxisEvents|InputAxisMoveForward
  (params (AxisValue :type Float%20%28single-precision%29))
  (Pawn|Input|AddMovementInput (Transformation|GetActorForwardVector) AxisValue false))

(fn ConstructionScript)