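; BP_IntersectionToRT is an actor that turns trace results into a texture shown on its own mesh, refreshed every frame.
; The construction script creates a dynamic material instance from a default material.
; Tick calls GenerateTrace and GenerateRTFromTrace, both defined outside this graph, then feeds the result into the DynamicTexture parameter and reapplies the material to the mesh.
; Debug nodes for printing and exporting the texture are left unconnected.
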(event EventBeginPlay)

(event Collision|EventActorBeginOverlap
  (params (OtherActor :type Actor%20Object%20Reference)))

(event EventTick
  (params (DeltaSeconds :type Float%20%28single-precision%29))
  (bind _mydynamicmaterial (Variables|Default|GetMyDynamicMaterial))
  (Class|IntersectiontoRT|GenerateTrace)
  (bind _generatedtexture (Class|IntersectiontoRT|GenerateRTfromTrace))
  (Rendering|Material|SetTextureParameterValue _mydynamicmaterial "DynamicTexture" _generatedtexture)
  (Rendering|Material|SetMaterial (Variables|Default|GetMeshComp) 0 _mydynamicmaterial))

(fn ConstructionScript
  (bind _returnvalue (Rendering|Material|CreateDynamicMaterialInstance "/Game/MyDefaultMat.MyDefaultMat" "MyDynamicMat" :!class /Script/Engine.KismetMaterialLibrary))
  (Variables|Default|SetMyDynamicMaterial _returnvalue))