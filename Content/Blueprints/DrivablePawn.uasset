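; Drivable boat pawn that the first player controller possesses on BeginPlay, driven with WASD and an orbiting look camera.
; Key gates set throttle and steering axes, which Tick turns into clamped force and a lerped wheel angle.
; Movement is hand-integrated velocity with damping and anti-slide, applied as unswept offsets, with yaw from steering and speed-scaled pitch and roll.
; The spring arm follows look input and optionally eases back after idle time.
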(event EventBeginPlay
  (bind _springarm (Variables|Default|GetSpringArm))
  (bind _relativerotation (Variables|/Script/Engine.SceneComponent|GetRelativeRotation _springarm))
  ;[1 1 1] Possess on BeginPlay
  (Pawn|Possess (Game|GetPlayerController 0) self)
  (Variables|Default|SetStartLookPitch (.pitch _relativerotation))
  (Variables|Default|SetCurrent%20Look%20Pitch (.pitch _relativerotation))
  (Variables|Default|SetCurrent%20Look%20Yaw (.yaw _relativerotation)))

(event Collision|EventActorBeginOverlap
  (params (OtherActor :type Actor%20Object%20Reference)))

(event EventTick
  (params (DeltaSeconds :type Float%20%28single-precision%29))
  (bind _returnvalue (Utilities|Time|GetWorldDeltaSeconds))
  (bind _acceleration (Variables|BoatSettings|GetAcceleration))
  (bind _pitchwhenmoving (Variables|BoatSettings|GetPitchWhenMoving))
  (bind _maxspeed (Variables|BoatSettings|GetMaxSpeed))
  (bind _currentsteeringwheel (Variables|Default|GetCurrentSteeringWheel))
  (bind _max_steer_angle (Variables|BoatSettings|GetMax%20Steer%20Angle))
  (bind _rootmesh (Variables|Default|GetRootMesh))
  (bind _returnvalue_2 (/ _acceleration 1.5))
  (Utilities|FlowControl|Sequence
    (:then_0
      ;[1 1 1] Calculate force
      (Variables|Default|SetCurrentForce (Math|Float|Clamp(Float) (+ (select (and (< (Variables|Default|GetCurrentForce) _returnvalue_2) (> (Variables|Default|GetCurrentForce) (* _returnvalue_2 -1.0))) 0.0 (select (> (Variables|Default|GetCurrentForce) 0.0) (- (Variables|Default|GetCurrentForce) _returnvalue_2) (+ (Variables|Default|GetCurrentForce) _returnvalue_2))) (* (Variables|Default|GetMoveForwardAxis) (Variables|BoatSettings|GetAcceleration))) (/ _maxspeed (Variables|BoatSettings|GetBackwardSpeedMultiplier)) _maxspeed))
      ;[1 1 1] Move boat
      (bind _output_get (Variables|Default|SetCurrent%20Horizontal%20Velocity (Math|Vector|MakeVector (.x (+ (+ (+ (Variables|Default|GetCurrent%20Horizontal%20Velocity) (* (Variables|Default|GetCurrent%20Horizontal%20Velocity) (* (Variables|BoatSettings|GetVelocityDamping) (Utilities|Time|GetWorldDeltaSeconds)))) (* (Transformation|GetActorRightVector) (* (* (Variables|Default|GetCurrent%20Sliding%20Speed) -1.0) (* (Variables|BoatSettings|GetAnti%20Slide) (Utilities|Time|GetWorldDeltaSeconds))))) (Math|Vector|MakeVector (.x (Math|Transform|TransformDirection (Transformation|GetWorldTransform (Variables|Default|GetRootMesh)) (* (Math|Vector|MakeVector (Variables|Default|GetCurrentForce) 0.0 0.0) (Utilities|Time|GetWorldDeltaSeconds)))) (.y (Math|Transform|TransformDirection (Transformation|GetWorldTransform (Variables|Default|GetRootMesh)) (* (Math|Vector|MakeVector (Variables|Default|GetCurrentForce) 0.0 0.0) (Utilities|Time|GetWorldDeltaSeconds)))) 0.0))) (.y (+ (+ (+ (Variables|Default|GetCurrent%20Horizontal%20Velocity) (* (Variables|Default|GetCurrent%20Horizontal%20Velocity) (* (Variables|BoatSettings|GetVelocityDamping) (Utilities|Time|GetWorldDeltaSeconds)))) (* (Transformation|GetActorRightVector) (* (* (Variables|Default|GetCurrent%20Sliding%20Speed) -1.0) (* (Variables|BoatSettings|GetAnti%20Slide) (Utilities|Time|GetWorldDeltaSeconds))))) (Math|Vector|MakeVector (.x (Math|Transform|TransformDirection (Transformation|GetWorldTransform (Variables|Default|GetRootMesh)) (* (Math|Vector|MakeVector (Variables|Default|GetCurrentForce) 0.0 0.0) (Utilities|Time|GetWorldDeltaSeconds)))) (.y (Math|Transform|TransformDirection (Transformation|GetWorldTransform (Variables|Default|GetRootMesh)) (* (Math|Vector|MakeVector (Variables|Default|GetCurrentForce) 0.0 0.0) (Utilities|Time|GetWorldDeltaSeconds)))) 0.0))) 0.0)))
      (Transformation|AddActorWorldOffset (* _output_get (Utilities|Time|GetWorldDeltaSeconds)))
      ;[1 1 1] Torque
      (CallFunction|UpdateMotorAngle)
      (Variables|Default|SetCurrentPitch (Math|Float|Clamp(Float) (Math|Float|Absolute(Float) (Math|Interpolation|FInterpTo (Variables|Default|GetCurrentPitch) (* _pitchwhenmoving (/ (Variables|Default|GetCurrent%20Horizontal%20Speed) (Variables|BoatSettings|GetMaxSpeed))) (Utilities|Time|GetWorldDeltaSeconds) 3.0)) 0.0 _pitchwhenmoving))
      (Variables|Default|SetCurrentRoll (Math|Float|Clamp(Float) (Math|Interpolation|FInterpTo (Variables|Default|GetCurrentRoll) (select (Math|Float|NearlyEqual(Float) _currentsteeringwheel 0.0 0.5) 0.0 (* (* (Variables|BoatSettings|GetRollWhenSteering) (/ _currentsteeringwheel (Variables|BoatSettings|GetMax%20Steer%20Angle))) (/ (Variables|Default|GetCurrent%20Horizontal%20Speed) (Variables|BoatSettings|GetMaxSpeed)))) (Utilities|Time|GetWorldDeltaSeconds) 3.0) (* -1 _max_steer_angle) _max_steer_angle))
      (Transformation|AddRelativeRotation _rootmesh (Math|Rotator|MakeRotator 0.0 0.0 (* (Variables|BoatSettings|GetSteeringForce) (Variables|Default|GetCurrentSteeringWheel) (Utilities|Time|GetWorldDeltaSeconds))) false false)
      (Transformation|SetActorRelativeRotation (Math|Rotator|MakeRotator (Variables|Default|GetCurrentRoll) (Variables|Default|GetCurrentPitch) (.yaw (Variables|/Script/Engine.SceneComponent|GetRelativeRotation _rootmesh))) false true))
    (:then_1
      ;[1 1 1] Rotate camera
      (if (Pawn|IsLocallyControlled)
        (Transformation|SetRelativeRotation (Variables|Default|GetSpringArm) (Math|Rotator|MakeRotator 0.0 (Variables|Default|GetCurrent%20Look%20Pitch) (Variables|Default|GetCurrent%20Look%20Yaw)) false false)
        (if (Variables|BoatSettings|GetMoveCameraBack)
          (if (or (!= (Input|AxisValues|GetLookRight) 0.0) (!= (Input|AxisValues|GetLookUp) 0.0))
            (Variables|Default|SetLookInputLastTime (Utilities|Time|GetTimeSeconds))
            (elif (>= (Utilities|Time|GetTimeSeconds) (+ (Variables|BoatSettings|GetSecondsBeforeResetLook) (Variables|Default|GetLookInputLastTime)))
              (Variables|Default|SetCurrent%20Look%20Pitch (Math|Interpolation|FInterpTo (Variables|Default|GetCurrent%20Look%20Pitch) (Variables|Default|GetStartLookPitch) _returnvalue 2.0))
              (Variables|Default|SetCurrent%20Look%20Yaw (Math|Interpolation|FInterpTo (Variables|Default|GetCurrent%20Look%20Yaw) 0.0 _returnvalue 2.0)))))))
    (:then_3
      ;[1 1 1] Calculate values
      (Variables|Default|SetCurrent%20Horizontal%20Speed (Math|Vector|VectorLength (Math|Vector|ProjectVectorontoPlane (* (- (Transformation|GetActorLocation) (Variables|Default|GetLastLocation)) (/ 1.0 (Utilities|Time|GetWorldDeltaSeconds))) (Math|Vector|GetUpVector (Variables|Default|GetRootMesh)))))
      (Variables|Default|SetCurrent%20Sliding%20Speed (Math|Vector|DotProduct (Variables|Default|GetCurrent%20Horizontal%20Velocity) (Transformation|GetActorRightVector)))
      (Variables|Default|SetLastLocation (Transformation|GetActorLocation)))))

(event Input|AxisEvents|InputAxisLookUp
  (params (AxisValue :type Float%20%28single-precision%29))
  ;[1 1 1] Look
  (Variables|Default|SetCurrent%20Look%20Pitch (Math|Float|Clamp(Float) (+ (Variables|Default|GetCurrent%20Look%20Pitch) (* (Math|Float|Clamp(Float) AxisValue -1.0) 5.0)) (Variables|BoatSettings|GetLookUpMin) (Variables|BoatSettings|GetLookUpMax))))

(event Input|AxisEvents|InputAxisLookRight
  (params (AxisValue :type Float%20%28single-precision%29))
  ;[1 1 1] Look
  (if (or (== (Math|Float|Clamp(Float) (+ (Variables|Default|GetCurrent%20Look%20Yaw) (* (Math|Float|Clamp(Float) AxisValue -1.0) 5.0)) -1.8e+02 1.8e+02) -1.8e+02) (== (Math|Float|Clamp(Float) (+ (Variables|Default|GetCurrent%20Look%20Yaw) (* (Math|Float|Clamp(Float) AxisValue -1.0) 5.0)) -1.8e+02 1.8e+02) 1.8e+02))
    (Variables|Default|SetCurrent%20Look%20Yaw (* (Math|Float|Clamp(Float) (+ (Variables|Default|GetCurrent%20Look%20Yaw) (* (Math|Float|Clamp(Float) AxisValue -1.0) 5.0)) -1.8e+02 1.8e+02) -1.0))
    (else
      (Variables|Default|SetCurrent%20Look%20Yaw (Math|Float|Clamp(Float) (+ (Variables|Default|GetCurrent%20Look%20Yaw) (* (Math|Float|Clamp(Float) AxisValue -1.0) 5.0)) -1.8e+02 1.8e+02)))))

(event Input|KeyboardEvents|S
  (params (Key :type Key%20Structure))
  ;[1 1 1] Input
  (:Pressed
    (Variables|Default|SetMoveForwardAxis -1.0)
    (Utilities|FlowControl|Gate false) ; enters at Close
  )
  (:Released
    (Utilities|FlowControl|Sequence
      (:then_0
        (Utilities|FlowControl|Gate false
          (:Exit
            (Variables|Default|SetMoveForwardAxis 0.0))))
      (:then_1
        (Utilities|FlowControl|Gate false) ; enters at Open
      ))))

(event Input|KeyboardEvents|A
  (params (Key :type Key%20Structure))
  ;[1 1 1] Input
  (:Pressed
    (Variables|Default|SetMoveRightAxis -1.0)
    (Utilities|FlowControl|Gate false) ; enters at Close
  )
  (:Released
    (Utilities|FlowControl|Sequence
      (:then_0
        (Utilities|FlowControl|Gate false
          (:Exit
            (Variables|Default|SetMoveRightAxis 0.0))))
      (:then_1
        (Utilities|FlowControl|Gate false) ; enters at Open
      ))))

(event Input|KeyboardEvents|W
  (params (Key :type Key%20Structure))
  ;[1 1 1] Input
  (:Pressed
    (Variables|Default|SetMoveForwardAxis 1.0)
    (Utilities|FlowControl|Gate false) ; enters at Close
  )
  (:Released
    (Utilities|FlowControl|Sequence
      (:then_0
        (Utilities|FlowControl|Gate false
          (:Exit
            (Variables|Default|SetMoveForwardAxis 0.0))))
      (:then_1
        (Utilities|FlowControl|Gate false) ; enters at Open
      ))))

(event Input|KeyboardEvents|D
  (params (Key :type Key%20Structure))
  ;[1 1 1] Input
  (:Pressed
    (Variables|Default|SetMoveRightAxis 1.0)
    (Utilities|FlowControl|Gate false) ; enters at Close
  )
  (:Released
    (Utilities|FlowControl|Sequence
      (:then_0
        (Utilities|FlowControl|Gate false
          (:Exit
            (Variables|Default|SetMoveRightAxis 0.0))))
      (:then_1
        (Utilities|FlowControl|Gate false) ; enters at Open
      ))))

(fn ConstructionScript)

(fn UpdateMotorAngle
  ;[1 1 1] Change steering wheel angle
  (Variables|Default|SetCurrentSteeringWheel (Math|Float|Lerp (Variables|Default|GetCurrentSteeringWheel) (* (Variables|Default|GetMoveRightAxis) (Variables|BoatSettings|GetMax%20Steer%20Angle)) (Math|Float|Clamp(Float) (* (Utilities|Time|GetWorldDeltaSeconds) (Variables|BoatSettings|GetSteeringChangingSpeed))))))