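; Buoyancy pawn prototype tied to a SimGrid, apparently meant to read simulation data at its location.
; BeginPlay only caches the grid's bounds size.
; Disconnected logic would update a buffer, sample a render target at the pawn's normalized grid position and print the blue channel.
; CheckBounds holds an XY containment test and relative-location calculation, both left unconnected.
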(event EventBeginPlay
  (bind _simgrid (Variables|Default|GetSimGrid))
  (bind _output_get (Variables|Default|SetSizeBound (- (Variables|/Game/SDFMethods/BP_Mat2RenderTarget.BP_Mat2RenderTarget_C|GetMaxBound _simgrid) (Variables|/Game/SDFMethods/BP_Mat2RenderTarget.BP_Mat2RenderTarget_C|GetMinBound _simgrid)))))

(event Collision|EventActorBeginOverlap
  (params (OtherActor :type Actor%20Object%20Reference)))

(event EventTick
  (params (DeltaSeconds :type Float%20%28single-precision%29)))

(fn ConstructionScript)